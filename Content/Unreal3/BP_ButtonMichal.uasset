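; Arcade-style in-world button that drives a claw, toggling its state or moving it according to an integer button type.
; Left clicks register only while the player overlaps its trigger and has the cursor on this button.
; Movement buttons run a very short timer that loops while pressed to move the claw.
; Releasing a holdable button, leaving the trigger or losing the cursor re-runs the handler to end the hold.
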(event `self.ReceiveBeginPlay`
  ; Get Player
  (bind _returnvalue (`GameplayStatics.GetActorOfClass` "/Game/FirstPerson/Blueprints/BP_FirstPersonCharacter.BP_FirstPersonCharacter_C"))
  (set `self.Player_BP` _returnvalue))

(event `Key|LeftMouseButton` :consume false
  (params (Key :type "Key Structure"))
  (bind _player_bp (`self.Player_BP`))
  ; Interaction
  (:`Pressed`
    (set `self.IsPressing` true)
    (if (`self.CanInteract`) :!label _label
      (if (`/Game/FirstPerson/Blueprints/BP_FirstPersonCharacter.CursorVisible` _player_bp)
        (if (== (`/Game/FirstPerson/Blueprints/BP_FirstPersonCharacter.ButtonVisible` _player_bp) self)
          (`self.HandleClickedEvents` :!label _label_2)))))
  (:`Released`
    (if (`self.IsPressing`)
      (set `self.IsPressing` false)
      (if (`self.IsButtonHoldable`)
        (goto _label)))))

(event `self.PlayerTrigger.OnComponentBeginOverlap`
  (params (OverlappedComponent :type "PrimitiveComponent Object Reference") (OtherActor :type "Actor Object Reference") (OtherComp :type "PrimitiveComponent Object Reference") (OtherBodyIndex :type Integer) (bFromSweep :type Boolean) (SweepResult :type "HitResult Structure (by ref)"))
  ; Interaction
  (cast `/Game/FirstPerson/Blueprints/BP_FirstPersonCharacter` OtherActor)
  (set `self.CanInteract` true))

(event `self.PlayerTrigger.OnComponentEndOverlap`
  (params (OverlappedComponent :type "PrimitiveComponent Object Reference") (OtherActor :type "Actor Object Reference") (OtherComp :type "PrimitiveComponent Object Reference") (OtherBodyIndex :type Integer))
  ; Interaction
  (cast `/Game/FirstPerson/Blueprints/BP_FirstPersonCharacter` OtherActor)
  (set `self.CanInteract` false)
  (set `self.IsPressing` false :!label _label_3) ; Simulate button release event on area leave
  (goto _label_2))

(event `OnCursorLeave`
  ; Interaction
  (goto _label_3))

(fn `HandleClawMove`
  (`/Game/Blueprints/BP_ClawArms.Move Claw` (`self.NewClaw_BP`) (`self.ButtonType`)))

(fn `HandleClickedEvents`
  (switch `int` (`self.ButtonType`) ; Split up claw movement to simulate arcade-ish feel
    (:`Default`
      (`KismetSystemLibrary.K2_SetTimer` null "HandleClawMove" 0.001 (`self.IsPressing`) true))
    (:`0`
      (if (`self.IsPressing`)
        (`/Game/Blueprints/BP_ClawArms.ChangeClawState` (`self.NewClaw_BP`))))))

(fn `UserConstructionScript`)