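; BP_Claw is a claw that grabs and releases BP_Item actors when E is pressed.
; The grab casts the actor from the Box begin-overlap event, checks its Cube against ItemCollider, eases it toward ItemSocket over time, then attaches it.
; Release detaches the item and restores gravity and physics simulation.
; The nodes that would disable gravity and physics on grab are unconnected.
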(event `Key|E`
  (params (Key :type "Key Structure"))
  (bind _itemsocket (`self.ItemSocket`))
  ; ClawGrab
  (:`Pressed`
    (bind _asbp_item (cast `/Game/Blueprints/BP_Item` (stale `self.Box.OnComponentBeginOverlap` OtherActor))
      (:`then`
        (if (`self.Is Attached`)
          (`SceneComponent.K2_DetachFromComponent` (`Actor.RootComponent` _asbp_item) "KeepWorld" "KeepWorld" "KeepWorld" true :!label _label)
          (set `self.Is Attached` false)
          (bind _cube (`/Game/Blueprints/BP_Item.Cube` _asbp_item))
          (`PrimitiveComponent.SetEnableGravity` _cube true)
          (`PrimitiveComponent.SetSimulatePhysics` _cube true)
          (else
            (bind _cube_2 (`/Game/Blueprints/BP_Item.Cube` _asbp_item))
            (if (`PrimitiveComponent.IsOverlappingComponent` _cube_2 (`self.ItemCollider`))
              (`KismetSystemLibrary.MoveComponentTo` (`/Game/Blueprints/BP_Item.Cube` _asbp_item) (`SceneComponent.K2_GetComponentLocation` _itemsocket) (`SceneComponent.K2_GetComponentRotation` _itemsocket) true true 1.0 true)
              (bind _returnvalue (`SceneComponent.K2_AttachToComponent` _cube_2 (`self.ItemSocket`) "None" "SnapToTarget" "SnapToTarget" "SnapToTarget" true))
              (set `self.Is Attached` _returnvalue)))))
      (:`CastFailed`
        (if (`self.Is Attached`)
          (goto _label))))))

(event `self.Box.OnComponentBeginOverlap`
  (params (OverlappedComponent :type "PrimitiveComponent Object Reference") (OtherActor :type "Actor Object Reference") (OtherComp :type "PrimitiveComponent Object Reference") (OtherBodyIndex :type Integer) (bFromSweep :type Boolean) (SweepResult :type "HitResult Structure (by ref)"))
  ; ClawGrab
)

(fn `UserConstructionScript`)