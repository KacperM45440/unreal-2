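; BP_Button is an interactable button that tells a claw Blueprint to grab an item when the player clicks near it.
; A PlayerTrigger overlap with the first-person character toggles a CanInteract flag, which gates the left mouse press.
; A valid press runs HandleClickedEvents, which calls GrabItem on the referenced ClawBP.
; The mouse input relies on Consume Input being disabled so multiple button instances can all react to clicks.
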(event `Key|LeftMouseButton` :consume false
  (params (Key :type "Key Structure"))
  ; Interaction
  (:`Pressed`
    (if (`self.CanInteract`)
      (`self.HandleClickedEvents`))))

(event `self.PlayerTrigger.OnComponentBeginOverlap`
  (params (OverlappedComponent :type "PrimitiveComponent Object Reference") (OtherActor :type "Actor Object Reference") (OtherComp :type "PrimitiveComponent Object Reference") (OtherBodyIndex :type Integer) (bFromSweep :type Boolean) (SweepResult :type "HitResult Structure (by ref)"))
  ; Interaction
  (cast `/Game/FirstPerson/Blueprints/BP_FirstPersonCharacter` OtherActor)
  (set `self.CanInteract` true))

(event `self.PlayerTrigger.OnComponentEndOverlap`
  (params (OverlappedComponent :type "PrimitiveComponent Object Reference") (OtherActor :type "Actor Object Reference") (OtherComp :type "PrimitiveComponent Object Reference") (OtherBodyIndex :type Integer))
  ; Interaction
  (cast `/Game/FirstPerson/Blueprints/BP_FirstPersonCharacter` OtherActor)
  (set `self.CanInteract` false))

(fn `HandleClickedEvents`
  (`/Game/Blueprints/BP_Claw.Grab Item` (`self.Claw_BP`)))

(fn `UserConstructionScript`)