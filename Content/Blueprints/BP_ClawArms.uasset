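; Physics-driven claw machine claw with three constrained arms on a pole that lowers, closes, raises, opens and returns to idle.
; ChangeClawState advances the state machine from Idle, Lowering or Raising; timers auto-advance Lowering, Closing and Opening, while Raising waits for another call.
; Helpers drive or reset constraint targets and physics velocities.
; HandleClawMove sweeps the root along a hard-coded direction, but nothing live here calls it.
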(event `self.ReceiveTick`
  (params (DeltaSeconds :type "Float (single-precision)"))
  ; DeltaTime
  (set `self.DeltaTime` DeltaSeconds))

(event `ChangeClawState`
  (bind _eclawstate (`self.EClawState`))
  (switch `/Game/Enums/Enum_ClawState` (`self.EClawState`)
    (:`NewEnumerator0`
      _)
    (:`NewEnumerator1`
      _)
    (:`NewEnumerator3`
      _))
  (`KismetSystemLibrary.K2_InvalidateTimerHandle` (stale _returnvalue))
  (`KismetSystemLibrary.PrintString` (`KismetStringLibrary.Conv_ByteToString` _eclawstate) :!label _label)
  (switch `/Game/Enums/Enum_ClawState` _eclawstate
    (:`NewEnumerator0`
      (bind _output_get (set `self.EClawState` "NewEnumerator1")))
    (:`NewEnumerator1`
      (set `self.EClawState` "NewEnumerator2"))
    (:`NewEnumerator2`
      (set `self.EClawState` "NewEnumerator3"))
    (:`NewEnumerator3`
      (set `self.EClawState` "NewEnumerator4"))
    (:`NewEnumerator4`
      (set `self.EClawState` "NewEnumerator0")))
  (switch `/Game/Enums/Enum_ClawState` _output_get
    (:`NewEnumerator0`
      (`self.ResetConstraintMovement` (`self.Arm1`) (`self.ArmConstraint1`))
      (`self.ResetConstraintMovement` (`self.Arm2`) (`self.ArmConstraint2`))
      (`self.ResetConstraintMovement` (`self.Arm3`) (`self.ArmConstraint3`))
      (`self.ResetConstraintMovement` (`self.OuterPole`) (`self.PoleConstraint`)))
    (:`NewEnumerator1`
      (`self.TogglePoleLowering` true)
      (set `self.TimerTemp` 5.0)
      (bind _returnvalue (`KismetSystemLibrary.K2_SetTimerDelegate` (delegate `AutomaticallyChangeState`) (`self.TimerTemp`) :!label _label_2)))
    (:`NewEnumerator2`
      (`self.ToggleArmGrab` (`self.Arm1`) (`self.ArmConstraint1`))
      (`self.ToggleArmGrab` (`self.Arm2`) (`self.ArmConstraint2`))
      (`self.ToggleArmGrab` (`self.Arm3`) (`self.ArmConstraint3`))
      (`self.ResetConstraintMovement` (`self.OuterPole`) (`self.PoleConstraint`))
      (set `self.TimerTemp` 1.5)
      (goto _label_2))
    (:`NewEnumerator3`
      (`self.TogglePoleLowering` false))
    (:`NewEnumerator4`
      (`self.ToggleArmGrab` (`self.Arm1`) (`self.ArmConstraint1`) true)
      (`self.ToggleArmGrab` (`self.Arm2`) (`self.ArmConstraint2`) true)
      (`self.ToggleArmGrab` (`self.Arm3`) (`self.ArmConstraint3`) true)
      (set `self.TimerTemp` 0.5)
      (goto _label_2))))

(event `AutomaticallyChangeState`
  (goto _label))

(event `self.HeadCollision.OnComponentBeginOverlap`
  (params (OverlappedComponent :type "PrimitiveComponent Object Reference") (OtherActor :type "Actor Object Reference") (OtherComp :type "PrimitiveComponent Object Reference") (OtherBodyIndex :type Integer) (bFromSweep :type Boolean) (SweepResult :type "HitResult Structure (by ref)")))

(event `self.ReceiveBeginPlay`)

(event `Key|LeftMouseButton` :consume false
  (params (Key :type "Key Structure")))

(fn `HandleClawMove`
  (locals (Direction :type "Float (double-precision)" :default 1.0))
  (bind _defaultsceneroot (`self.DefaultSceneRoot`))
  (bind _deltatime (`self.DeltaTime`))
  (bind _returnvalue (`SceneComponent.K2_GetComponentLocation` _defaultsceneroot))
  ; Move Claw
  (switch `int` 2 ; 1 - Left, 2 - Up, 3 - Right, 4 - Down
    (:`1`
      (bind _output_get (set `self.AxisModifier` -100.0))
      (set `self.NewLocation` (+ _returnvalue (`KismetMathLibrary.MakeVector` 0.0 (* _deltatime _output_get)))))
    (:`2`
      (bind _output_get_2 (set `self.AxisModifier` 100.0))
      (set `self.NewLocation` (+ _returnvalue (`KismetMathLibrary.MakeVector` (* _deltatime _output_get_2)))))
    (:`3`
      (bind _output_get_3 (set `self.AxisModifier` 100.0))
      (set `self.NewLocation` (+ _returnvalue (`KismetMathLibrary.MakeVector` 0.0 (* _deltatime _output_get_3)))))
    (:`4`
      (bind _output_get_4 (set `self.AxisModifier` -100.0))
      (set `self.NewLocation` (+ _returnvalue (`KismetMathLibrary.MakeVector` (* _deltatime _output_get_4))))))
  (`SceneComponent.K2_SetWorldLocation` _defaultsceneroot (`self.NewLocation`) true false))

(fn `ResetConstraintMovement`
  (params (Mesh :type "StaticMeshComponent Object Reference") (Constraint :type "PhysicsConstraintComponent Object Reference"))
  (`PrimitiveComponent.SetPhysicsLinearVelocity` Mesh (0.0 0.0 0.0) false "None")
  (`PrimitiveComponent.SetPhysicsAngularVelocityInDegrees` Mesh (0.0 0.0 0.0) false "None")
  (`PhysicsConstraintComponent.SetLinearPositionTarget` Constraint (`SceneComponent.K2_GetComponentLocation` Constraint))
  (`PhysicsConstraintComponent.SetAngularOrientationTarget` Constraint (`SceneComponent.K2_GetComponentRotation` Constraint)))

(fn `ToggleArmGrab`
  (params (ArmMesh :type "StaticMeshComponent Object Reference") (ArmConstraint :type "PhysicsConstraintComponent Object Reference") (Open :type Boolean))
  (locals (Rotation :type "Float (single-precision)" :default 20.0))
  (`PrimitiveComponent.SetPhysicsAngularVelocityInDegrees` ArmMesh (0.0 0.0 0.0) false "None")
  (if Open
    (set `local.Rotation` (`self.OpenRotation`))
    (else
      (set `local.Rotation` (`self.ClosedRotation`))))
  (`PhysicsConstraintComponent.SetAngularOrientationTarget` ArmConstraint (`KismetMathLibrary.MakeRotator` (`local.Rotation`))))

(fn `TogglePoleLowering`
  (params (Lowering :type Boolean))
  (locals (Position :type "Float (double-precision)"))
  (bind _outerpole (`self.OuterPole`))
  (if Lowering
    (`PrimitiveComponent.SetPhysicsLinearVelocity` _outerpole (0.0 0.0 -1.0) false "None")
    (set `local.Position` (`self.LoweringPosition`))
    (else
      (`PrimitiveComponent.SetPhysicsLinearVelocity` _outerpole (0.0 0.0 1.0) false "None")
      (set `local.Position` (`self.RaisingPosition`))))
  (`PhysicsConstraintComponent.SetLinearPositionTarget` (`self.PoleConstraint`) (`KismetMathLibrary.MakeVector` 0.0 0.0 (`local.Position`))))

(fn `UserConstructionScript`)